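; Blue pressure plate that opens its linked door when an overlapping base, red or blue cube has a color ID matching the plate's.
; A match sets the plate active, lowers its mesh through a timeline and opens DoorToOpen.
; Any end overlap closes the door and clears IsActive before calling Inactive, whose raise timeline requires that flag, so that animation is skipped.
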(event `self.ReceiveActorBeginOverlap`
  (params (OtherActor :type "Actor Object Reference"))
  (`self.If Plate Id Equals Cube Id Open Door` OtherActor))

(event `self.ReceiveActorEndOverlap`
  (params (OtherActor :type "Actor Object Reference"))
  (`self.CloseDoor`))

(event `Active`
  ;[1 1 1] Play Animation
  (if (`self.IsActive`)
    (bind (_direction _godown) (`Timeline|Timeline`)
      (:`Update`
        (`SceneComponent.K2_SetRelativeLocation` (`self.Plate`) (`KismetMathLibrary.MakeVector` 0.0 0.0 (`|EaseFunction` "Linear" _godown 0.0 -3.5)) false false)))))

(event `Inactive`
  ;[1 1 1] Play Animation
  (if (`self.IsActive`)
    (bind (_direction _godown) (`Timeline|Timeline_0`)
      (:`Update`
        (`SceneComponent.K2_SetRelativeLocation` (`self.Plate`) (`KismetMathLibrary.MakeVector` 0.0 0.0 (`|EaseFunction` "Linear" _godown 0.0 2.0)) false false)))))

(fn `CloseDoor`
  (set `self.IsActive` false)
  (`self.Inactive`)
  (`/Game/MyAssets/Blueprints/BP_BaseDoor.Close` (`self.DoorToOpen`)))

(fn `If Plate Id Equals Cube Id Open Door`
  (params (Object :type "Object Object Reference"))
  (bind _asbp_base_cube (cast `/Game/MyAssets/Blueprints/BP_BaseCube` Object)
    (:`then`
      (for _array_element (`|MakeArray` _asbp_base_cube)
        (if (== (`/Game/MyAssets/Blueprints/BP_BaseCube.CubeColorID` _array_element) (`self.PlateColorID`))
          (set `self.IsActive` true)
          (`self.Active`)
          (`/Game/MyAssets/Blueprints/BP_BaseDoor.Open` (`self.DoorToOpen`)))))
    (:`CastFailed`
      (bind _asbp_red_cube (cast `/Game/MyAssets/Blueprints/BP_RedCube` Object)
        (:`then`
          (for _array_element_2 (`|MakeArray` _asbp_red_cube)
            (if (== (`/Game/MyAssets/Blueprints/BP_RedCube.CubeColorID` _array_element_2) (`self.PlateColorID`))
              (set `self.IsActive` true)
              (`self.Active`)
              (`/Game/MyAssets/Blueprints/BP_BaseDoor.Open` (`self.DoorToOpen`)))))
        (:`CastFailed`
          (bind _asbp_blue_cube (cast `/Game/MyAssets/Blueprints/BP_BlueCube` Object))
          (for _array_element_3 (`|MakeArray` _asbp_blue_cube)
            (if (== (`/Game/MyAssets/Blueprints/BP_BlueCube.CubeColorID` _array_element_3) (`self.PlateColorID`))
              (set `self.IsActive` true)
              (`self.Active`)
              (`/Game/MyAssets/Blueprints/BP_BaseDoor.Open` (`self.DoorToOpen`)))))))))

(fn `UserConstructionScript`)